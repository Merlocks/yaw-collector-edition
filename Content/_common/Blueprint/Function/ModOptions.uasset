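; Blueprint function library that exposes mod options stored in a custom config section for the YAW Collector Edition mod.
; GetTraceRangeMultiplier reads a trace range multiplier through Victory plugin config functions and clamps it to a safe range.
; When the setting is missing, it writes a neutral default to the config and returns that value.
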(fn `GetConfigSection`
  (returns (NewParam :type String))
  (return "YAWCollectorEdition"))

(fn `GetTraceRangeMultiplier`
  (returns (float :type "Float (double-precision)"))
  (locals (ConfigSection :type String))
  (bind (_isvalid _returnvalue) (`VictoryBPFunctionLibrary.VictoryGetCustomConfigVar_Float` (`local.ConfigSection`) "fTraceRangeMult"))
  (set `local.ConfigSection` (`self.GetConfigSection` null))
  (if _isvalid
    (return (`KismetMathLibrary.FClamp` _returnvalue 0.0 2.0))
    (else
      (`VictoryBPFunctionLibrary.VictorySetCustomConfigVar_Float` (`local.ConfigSection`) "fTraceRangeMult" 1.0)
      (return 1.0))))